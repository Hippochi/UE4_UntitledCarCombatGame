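; Projectile-like actor that destroys itself on contact and damages turrets.
; Its StaticMesh overlap event checks the other component's object type, destroying the actor on WorldDynamic, WorldStatic or the first custom game channel.
; On the custom channel it also casts the other actor to BP_TURRET, lowers its Helf by a fixed amount and plays a collapse sound at the world origin.
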(event OnComponentBeginOverlap(StaticMesh)
  (params (OverlappedComponent :type Primitive%20Component%20Object%20Reference) (OtherActor :type Actor%20Object%20Reference) (OtherComp :type Primitive%20Component%20Object%20Reference) (OtherBodyIndex :type Integer) (bFromSweep :type Boolean) (SweepResult :type Hit%20Result%20Structure%20%28by%20ref%29))
  (bind _returnvalue (Collision|GetCollisionObjectType OtherComp))
  (if (Utilities|Enum|Equal(Enum) _returnvalue "ECC_WorldDynamic")
    (Actor|DestroyActor :!label _label)
    (elif (Utilities|Enum|Equal(Enum) _returnvalue "ECC_WorldStatic")
      (goto _label)
      (elif (Utilities|Enum|Equal(Enum) _returnvalue "ECC_GameTraceChannel1")
        (Actor|DestroyActor)
        (bind _asbp_turret (Utilities|Casting|CastToBP_TURRET OtherActor))
        (Variables|/Game/Turret/BP_TURRET.BP_TURRET_C|Sethelf _asbp_turret (- (Variables|/Game/Turret/BP_TURRET.BP_TURRET_C|Gethelf _asbp_turret) 0.5))
        (Audio|PlaySoundatLocation "/Game/StarterContent/Audio/Collapse02.Collapse02" "0, 0, 0" "0, 0, 0" 1.0 1.0 0.0 0 0 0)))))

(event EventBeginPlay)

(event Collision|EventActorBeginOverlap
  (params (OtherActor :type Actor%20Object%20Reference)))

(event EventTick
  (params (DeltaSeconds :type Float%20%28single-precision%29)))

(fn ConstructionScript)
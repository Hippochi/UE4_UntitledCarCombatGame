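; BP_TURRET is an enemy turret that tracks and shoots the player while they are inside its Box trigger.
; Tick slowly interpolates the barrel toward the target, slightly above its location.
; Overlap starts or clears a looping fire timer, which spawns BP_Projectile with a sound only when a muzzle line trace hits the target.
; When Helf runs out, it destroys itself and decrements Turrets on the BP_Pickup player pawn.
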(event OnComponentBeginOverlap(Box)
  (params (OverlappedComponent :type Primitive%20Component%20Object%20Reference) (OtherActor :type Actor%20Object%20Reference) (OtherComp :type Primitive%20Component%20Object%20Reference) (OtherBodyIndex :type Integer) (bFromSweep :type Boolean) (SweepResult :type Hit%20Result%20Structure%20%28by%20ref%29))
  (if (not (Variables|Default|GetHasTarget))
    (if (== OtherActor (Game|Player|GetPlayerPawn 0))
      (Variables|Default|SetTargetPawn OtherActor)
      (Variables|Default|SetHasTarget true)
      (bind _returnvalue (Utilities|Time|SetTimerbyEvent (delegate Custom|fire) 1.5 true))
      (Variables|Default|SettimerHandle _returnvalue)
      (Transformation|SetWorldRotation (Variables|Default|GetTurretBarrel) (Math|Rotator|MakeRotfromX (Math|Interpolation|VInterpTo (Math|Rotator|GetRotationXVector (Transformation|GetWorldRotation (Variables|Default|GetTurretBarrel))) (+ (- (Transformation|GetActorLocation (Variables|Default|GetTargetPawn)) (Transformation|GetWorldLocation (Variables|Default|GetTurretBarrel))) "0,0.000000,100.000000") (stale EventTick DeltaSeconds) 0.01)) false false))))

(event OnComponentEndOverlap(Box)
  (params (OverlappedComponent :type Primitive%20Component%20Object%20Reference) (OtherActor :type Actor%20Object%20Reference) (OtherComp :type Primitive%20Component%20Object%20Reference) (OtherBodyIndex :type Integer))
  (if (== OtherActor (Game|Player|GetPlayerPawn 0))
    (if (Variables|Default|GetHasTarget)
      (Variables|Default|SetHasTarget false)
      (Utilities|Time|ClearandInvalidateTimerbyHandle (Variables|Default|GettimerHandle)))))

(event Custom|fire
  (bind _visible_ (CallFunction|IsTargetVisible))
  (if _visible_
    (CallFunction|FireProj)
    (Audio|PlaySoundatLocation "/Game/Turret/SFX/212607__pgi__machine-gun-002-single-shot.212607__pgi__machine-gun-002-single-shot" "0, 0, 0" "0, 0, 0" 0.4 1.0 0.0 0 0 0)))

(event EventTick
  (params (DeltaSeconds :type Float%20%28single-precision%29))
  (if (> (Variables|Default|Gethelf) 0.0)
    (if (Variables|Default|GetHasTarget)
      (Transformation|SetWorldRotation (Variables|Default|GetTurretBarrel) (Math|Rotator|MakeRotfromX (Math|Interpolation|VInterpTo (Math|Rotator|GetRotationXVector (Transformation|GetWorldRotation (Variables|Default|GetTurretBarrel))) (+ (- (Transformation|GetActorLocation (Variables|Default|GetTargetPawn)) (Transformation|GetWorldLocation (Variables|Default|GetTurretBarrel))) "0,0.000000,100.000000") DeltaSeconds 0.01)) false false))
    (else
      (Actor|DestroyActor)
      (bind _asbp_pickup (Utilities|Casting|CastToBP_Pickup (Game|Player|GetPlayerPawn 0)))
      (Math|Integer|DecrementInt (Variables|/Game/GameVehicles/Blueprints/Pickup/BP_Pickup.BP_Pickup_C|GetTurrets _asbp_pickup)))))

(fn ConstructionScript)

(fn IsTargetVisible
  (bind _turretbarrel (Variables|Default|GetTurretBarrel))
  (bind _returnvalue (Transformation|GetSocketTransform _turretbarrel "muzzle" "RTS_World"))
  (bind _outhit (Collision|LineTraceByChannel (.location _returnvalue) (+ (.location _returnvalue) (* (Math|Rotator|GetRotationXVector (.rotation _returnvalue)) (Variables|Default|Getrange))) "TraceTypeQuery1" false 0 "ForOneFrame"))
  (return (== (.HitActor (Collision|BreakHitResult _outhit)) (Variables|Default|GetTargetPawn))))

(fn FireProj
  (bind _turretbarrel (Variables|Default|GetTurretBarrel))
  (bind _returnvalue (Transformation|GetSocketRotation _turretbarrel "muzzle"))
  (Game|SpawnActorfromClass "/Game/Turret/BP_Projectile.BP_Projectile_C" (Math|Transform|MakeTransform (+ (Transformation|GetSocketLocation _turretbarrel "muzzle") (Math|Vector|RotateVector "5.000000, 0,0.000000" _returnvalue)) _returnvalue) "Undefined" self 0))
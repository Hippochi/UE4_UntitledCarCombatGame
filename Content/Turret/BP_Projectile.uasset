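; BP_Projectile is a turret projectile that damages a BP_Pickup on contact.
; Its Sphere overlap checks the other component's object type and destroys the projectile on Vehicle or WorldStatic hits.
; On a Vehicle hit it also casts the actor to BP_Pickup, subtracts a fixed amount from its Helf variable and plays an explosion sound at the world origin rather than the impact point.
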(event OnComponentBeginOverlap(Sphere)
  (params (OverlappedComponent :type Primitive%20Component%20Object%20Reference) (OtherActor :type Actor%20Object%20Reference) (OtherComp :type Primitive%20Component%20Object%20Reference) (OtherBodyIndex :type Integer) (bFromSweep :type Boolean) (SweepResult :type Hit%20Result%20Structure%20%28by%20ref%29))
  (if (Utilities|Enum|Equal(Enum) (Collision|GetCollisionObjectType OtherComp) "ECC_Vehicle")
    (Actor|DestroyActor)
    (bind _asbp_pickup (Utilities|Casting|CastToBP_Pickup OtherActor))
    (Variables|/Game/GameVehicles/Blueprints/Pickup/BP_Pickup.BP_Pickup_C|SetHelf _asbp_pickup (- (Variables|/Game/GameVehicles/Blueprints/Pickup/BP_Pickup.BP_Pickup_C|GetHelf _asbp_pickup) 0.11))
    (Audio|PlaySoundatLocation "/Game/StarterContent/Audio/Explosion01.Explosion01" "0, 0, 0" "0, 0, 0" 1.0 1.0 0.0 0 0 0)
    (elif (Utilities|Enum|Equal(Enum) (Collision|GetCollisionObjectType OtherComp) "ECC_WorldStatic")
      (Actor|DestroyActor))))

(fn ConstructionScript)